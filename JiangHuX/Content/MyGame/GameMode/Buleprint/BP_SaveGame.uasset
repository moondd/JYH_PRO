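; Save-game Blueprint that holds guild state, including characters, inter-guild friendship and which guilds are inside each guild.
; NewSaveData fills GuildDataArray from DT_GuildData, using numeric row names as indices and randomizing Dominate plus each character's Camp and Moral.
; One guild type also gets an action-time entry and is registered inside itself.
; Helpers apply friendship changes symmetrically to both guilds, read those values and add or remove contained guild IDs.
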(event `NewSaveData`
  (`self.ResetGuildDataArray`))

(fn `GetGuildFriendValue`
  (params (InGuildID :type Integer) (TargetGuildID :type Integer))
  (returns (OutGuildFriendValue :type Integer))
  (return (`|GetArrayItem` (`.GuildFriendValueArray_90_25B164BE4E691FB5E21701B217BD373D` (break `/Game/MyGame/GameMode/GameData/S_GuildData` (`|GetArrayItem` (`self.GuildDataArray`) InGuildID))) TargetGuildID)))

(fn `ResetGuildDataArray`
  (bind _guilddataarray (`self.GuildDataArray`))
  (bind _outrownames (`DataTableFunctionLibrary.GetDataTableRowNames` "/Game/MyGame/GameMode/GameData/DT_GuildData.DT_GuildData"))
  (for _array_element _outrownames
    (bind _returnvalue (`|GetDataTableRow` "/Game/MyGame/GameMode/GameData/DT_GuildData.DT_GuildData" _array_element)
      (:`then`
        (bind _returnvalue_2 (`KismetStringLibrary.Conv_StringToInt` (`KismetStringLibrary.Conv_NameToString` _array_element)))
        (bind (_guildtype _name _ap _dominate _parentguildid _characterdataarray _guildwar _guildfriendvaluearray _currguildaction _guildcolor _otherguildinthis _faith _quest) (break `/Game/MyGame/GameMode/GameData/S_GuildData` _returnvalue))
        (`KismetArrayLibrary.Array_Set` _guilddataarray _returnvalue_2 (make `/Game/MyGame/GameMode/GameData/S_GuildData` _guildtype _name _ap (`KismetMathLibrary.RandomIntegerInRange` 0 100) _parentguildid _characterdataarray _guildwar _guildfriendvaluearray _currguildaction _guildcolor _otherguildinthis _faith _quest) true)
        (bind _output (`|GetArrayItem` _guilddataarray _returnvalue_2))
        (bind (_guildtype_2 _name_2 _ap_2 _dominate_2 _parentguildid_2 _characterdataarray_2) (break `/Game/MyGame/GameMode/GameData/S_GuildData` _output))
        (for (_ _array_index) _characterdataarray_2
          (setmembers `/Game/MyGame/GameMode/GameData/S_GuildData` :`StructRef` _output :`CurrGuildAction` (make `/Game/MyGame/GameMode/GameData/S_GuildAction` _returnvalue_2 _returnvalue_2))
          (setmembers `/Game/MyGame/GameMode/GameData/S_CharacterData` :`StructRef` (`|GetArrayItem` _characterdataarray_2 _array_index) :`Camp` (cast `/Game/MyGame/GameMode/GameData/E_Camp` (`KismetMathLibrary.Conv_IntToByte` (`KismetMathLibrary.RandomIntegerInRange` 0 2))) :`Moral` (cast `/Game/MyGame/GameMode/GameData/E_Moral` (`KismetMathLibrary.Conv_IntToByte` (`KismetMathLibrary.RandomIntegerInRange` 0 2)))))
        (if (`|EnumEquality` (`.GuildType_78_7D1724C94388B20F680A0DB6A0D8995C` (break `/Game/MyGame/GameMode/GameData/S_GuildData` _returnvalue)) "NewEnumerator2")
          (`BlueprintMapLibrary.Map_Add` (`self.AllGuildActionTimeMap`) _returnvalue_2 (`KismetMathLibrary.MakeDateTime` 0))
          (`self.SetGuildIDToInGuildArray` _returnvalue_2 _returnvalue_2))))))

(fn `SetGuildFriendValue`
  (params (InGuildID :type Integer) (InOtherGuildID :type Integer) (InAddValue :type Integer))
  (locals (LocalVar_GuildID :type Integer) (LocalVar_TargetGuildID :type Integer) (LocalVar_AddValue :type Integer))
  (bind _localvar_targetguildid (`local.LocalVar_TargetGuildID`))
  (bind _localvar_guildid (`local.LocalVar_GuildID`))
  (bind _localvar_addvalue (`local.LocalVar_AddValue`))
  (bind (_guildtype _name _ap _dominate _parentguildid _characterdataarray _guildwar _guildfriendvaluearray) (break `/Game/MyGame/GameMode/GameData/S_GuildData` (`|GetArrayItem` (`self.GuildDataArray`) (`local.LocalVar_TargetGuildID`))))
  (bind (_guildtype_2 _name_2 _ap_2 _dominate_2 _parentguildid_2 _characterdataarray_2 _guildwar_2 _guildfriendvaluearray_2) (break `/Game/MyGame/GameMode/GameData/S_GuildData` (`|GetArrayItem` (`self.GuildDataArray`) (`local.LocalVar_GuildID`))))
  (set `local.LocalVar_GuildID` InGuildID)
  (set `local.LocalVar_TargetGuildID` InOtherGuildID)
  (set `local.LocalVar_AddValue` InAddValue)
  (if (`KismetArrayLibrary.Array_IsValidIndex` _guildfriendvaluearray_2 _localvar_targetguildid)
    (`KismetArrayLibrary.Array_Set` _guildfriendvaluearray_2 _localvar_targetguildid (+ (`|GetArrayItem` _guildfriendvaluearray_2 _localvar_targetguildid) _localvar_addvalue) true)
    (else
      (`KismetArrayLibrary.Array_Set` _guildfriendvaluearray_2 _localvar_targetguildid (`local.LocalVar_AddValue`) true)))
  (if (`KismetArrayLibrary.Array_IsValidIndex` _guildfriendvaluearray _localvar_guildid)
    (`KismetArrayLibrary.Array_Set` _guildfriendvaluearray _localvar_guildid (+ (`|GetArrayItem` _guildfriendvaluearray _localvar_guildid) _localvar_addvalue) true)
    (else
      (`KismetArrayLibrary.Array_Set` _guildfriendvaluearray _localvar_guildid (`local.LocalVar_AddValue`) true)))
  (return))

(fn `SetGuildIDToInGuildArray`
  (params (InGuildID :type Integer) (InTargetGuildID :type Integer) (Remove :type Boolean))
  (bind (_guildtype _name _ap _dominate _parentguildid _characterdataarray _guildwar _guildfriendvaluearray _currguildaction _guildcolor _otherguildinthis) (break `/Game/MyGame/GameMode/GameData/S_GuildData` (`|GetArrayItem` (`self.GuildDataArray`) InTargetGuildID)))
  (if Remove
    (if (`KismetArrayLibrary.Array_Contains` _otherguildinthis InGuildID)
      (`KismetArrayLibrary.Array_RemoveItem` _otherguildinthis InGuildID))
    (else
      (`KismetArrayLibrary.Array_Add` _otherguildinthis InGuildID))))