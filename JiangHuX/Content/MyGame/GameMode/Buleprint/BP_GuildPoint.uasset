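; BP_GuildPoint is a world-map guild location that reports player entry and exit to BP_GameMode_WorldMap and spawns the guild's AI characters.
; Construction collects move points from actors tagged with its GuildID.
; AddCharacterInThisGuild spawns living, not-yet-registered Native or Mission characters at the entrance or move points, assigning fixed routes or free roaming, optionally as a team.
; BuildGuildShpere tints and scales the sphere, then ground-snaps the actor by line trace.
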(event `self.ReceiveBeginPlay`)

(event `self.ReceiveActorBeginOverlap`
  (params (OtherActor :type "Actor Object Reference")))

(event `self.ReceiveTick`
  (params (DeltaSeconds :type "Float (single-precision)")))

(event `self.Event_PlayerIn`
  (`parent.Event_PlayerIn`)
  (bind _asbp_game_mode_world_map (cast `/Game/MyGame/GameMode/Buleprint/BP_GameMode_WorldMap` (`GameplayStatics.GetGameMode`)))
  (if (!= (`/Game/MyGame/GameMode/Buleprint/BP_GameMode_WorldMap.CurrGuildPoint` _asbp_game_mode_world_map) self)
    (`/Game/MyGame/GameMode/Buleprint/BP_GameMode_WorldMap.Event_PlayerEnterGuildPoint` _asbp_game_mode_world_map self)
    (`KismetSystemLibrary.PrintString` (`KismetStringLibrary.JoinStringArray` (`|MakeArray` "进入" "Guild" (`KismetStringLibrary.Conv_IntToString` (`self.GuildID`)))))))

(event `self.Event_PlayerLeave`
  (bind _asbp_game_mode_world_map (cast `/Game/MyGame/GameMode/Buleprint/BP_GameMode_WorldMap` (`GameplayStatics.GetGameMode`)))
  (if (== (`/Game/MyGame/GameMode/Buleprint/BP_GameMode_WorldMap.CurrGuildPoint` _asbp_game_mode_world_map) self)
    (`/Game/MyGame/GameMode/Buleprint/BP_GameMode_WorldMap.Event_PlayerLeaveGuildPoint` _asbp_game_mode_world_map self)
    (`KismetSystemLibrary.PrintString` (`KismetStringLibrary.JoinStringArray` (`|MakeArray` "离开" "Guild" (`KismetStringLibrary.Conv_IntToString` (`self.GuildID`)))))))

(fn `AddCharacterInThisGuild`
  (params (GuildID :type Integer) (Native :type Boolean) (Mission :type Boolean) (IsTeam :type Boolean) (InEntrance :type Boolean))
  (locals (Loc_Character_Count_First :type Integer) (Loc_Character_Count_Last :type Integer) (Loc_CharacterGuildID :type Integer) (Loc_CharacterBaseArray :type "Array of /Game/MyGame/GameMode/Character/JYH_BP_Character_Base Object Reference") (GameMode :type "/Game/MyGame/GameMode/Buleprint/BP_GameMode_WorldMap Object Reference"))
  (bind _aifixedpointarrayarray (`self.AIFixedPointArrayArray`))
  (bind _loc_characterguildid (`local.Loc_CharacterGuildID`))
  (bind _loc_characterbasearray (`local.Loc_CharacterBaseArray`))
  (`|ExecutionSequence`
    (:`then_0`
      (set `local.Loc_CharacterGuildID` GuildID)
      (bind _asbp_game_mode_world_map (cast `/Game/MyGame/GameMode/Buleprint/BP_GameMode_WorldMap` (`GameplayStatics.GetGameMode`)))
      (set `local.GameMode` _asbp_game_mode_world_map))
    (:`then_1`
      (for (_array_element _array_index) (`.CharacterDataArray_77_471FFE724D5A30DA053F2387D6E7B8C9` (break `/Game/MyGame/GameMode/GameData/S_GuildData` (`/Game/MyGame/GameMode/Buleprint/BP_FunctionLibrary.GetGuildDataWithID` (`local.Loc_CharacterGuildID`))))
        (if (and (`self.IsCharacterCanAdd` _array_element Mission Native) (not (`BlueprintMapLibrary.Map_Contains` (`/Game/MyGame/GameMode/Buleprint/BP_GameMode_WorldMap.AllCharacterAIArray` (`local.GameMode`)) (`KismetStringLibrary.JoinStringArray` (`|MakeArray` (`KismetStringLibrary.Conv_IntToString` (`local.Loc_CharacterGuildID`)) (`KismetStringLibrary.Conv_IntToString` _array_index)) ","))))
          (bind _returnvalue (`AIBlueprintHelperLibrary.SpawnAIFromClass` "/Game/MyGame/GameMode/Character/JYH_BP_Character_AI.JYH_BP_Character_AI_C" null (0.0 0.0 0.0) (struct) true))
          (bind _asjyh_bp_character_ai (cast `/Game/MyGame/GameMode/Character/JYH_BP_Character_AI` _returnvalue))
          (`KismetArrayLibrary.Array_Add` (`Actor.Tags` _asjyh_bp_character_ai) (`KismetStringLibrary.Conv_StringToName` (`KismetStringLibrary.Conv_IntToString` (`local.Loc_CharacterGuildID`))))
          (if (and (== (`self.GuildID`) (`local.Loc_CharacterGuildID`)) (`KismetArrayLibrary.Array_IsValidIndex` _aifixedpointarrayarray _array_index))
            (`/Game/MyGame/GameMode/Character/JYH_BP_Character_AI.SetCharacterAIConfig` _asjyh_bp_character_ai (`.ActorArray_5_D8261D6E4B283D939267F7BAD32CEC99` (break `/Game/MyGame/GameMode/GameData/S_ActorArray` (`|GetArrayItem` _aifixedpointarrayarray _array_index))) self false _loc_characterguildid _array_index)
            (else
              (`/Game/MyGame/GameMode/Character/JYH_BP_Character_AI.SetCharacterAIConfig` _asjyh_bp_character_ai (`self.MovePointArray`) self true _loc_characterguildid _array_index)))
          (`self.K2_SetActorTransform` _asjyh_bp_character_ai (`KismetMathLibrary.MakeTransform` (+ (`KismetMathLibrary.SelectVector` (`self.FindEntranceLocation`) (`self.SelectNewCharacterLocation`) InEntrance) (0.0 0.0 300.0))) false false)
          (`KismetArrayLibrary.Array_Add` (`local.Loc_CharacterBaseArray`) _asjyh_bp_character_ai)
          (bind _asbp_game_mode_world_map_2 (cast `/Game/MyGame/GameMode/Buleprint/BP_GameMode_WorldMap` (`GameplayStatics.GetGameMode`)))
          (`/Game/MyGame/GameMode/Buleprint/BP_GameMode_WorldMap.Event_CharacterEnter` _asbp_game_mode_world_map_2 _asjyh_bp_character_ai)))
      (if IsTeam
        (for _array_element_2 _loc_characterbasearray
          (set `/Game/MyGame/GameMode/Character/JYH_BP_Character_Base.Team` _loc_characterbasearray _array_element_2))))))

(fn `BuildGuildShpere`
  (params (LinearColor :type "LinearColor Structure (by ref)") (ScaleValue :type "Float (double-precision)"))
  (bind _returnvalue (`self.K2_GetActorLocation`))
  (bind _sphere (`self.Sphere`))
  (`PrimitiveComponent.SetMaterial` _sphere 0 "/Game/MyGame/GameMode/Material/M_GuildSphere_Base_Inst.M_GuildSphere_Base_Inst")
  (`MeshComponent.SetVectorParameterValueOnMaterials` _sphere "MainColor" (`KismetMathLibrary.Conv_LinearColorToVector` LinearColor))
  (`SceneComponent.SetRelativeScale3D` _sphere (`KismetMathLibrary.MakeVector` ScaleValue ScaleValue ScaleValue))
  (bind (_outhit _returnvalue_2) (`KismetSystemLibrary.LineTraceSingleForObjects` _returnvalue (`KismetMathLibrary.MakeVector` (.x _returnvalue) (+ (.y _returnvalue) 0.05) -30000.0) (`|MakeArray` "ObjectTypeQuery1" :!type "EObjectTypeQuery Enum") false (`|MakeArray` null :!type "Actor Object Reference")))
  (if _returnvalue_2
    (`self.K2_SetActorLocation` (`.Location` (`GameplayStatics.BreakHitResult` _outhit)))
    (else
      (`KismetSystemLibrary.PrintString` "Hello"))))

(fn `FindEntranceLocation`
  (returns (Location :type "Vector Structure"))
  (bind _entrancearray (`self.EntranceArray`))
  (bind _output (`|GetArrayItem` _entrancearray))
  (if (> (`KismetArrayLibrary.Array_Length` _entrancearray) 0)
    (if (`KismetSystemLibrary.IsValid` _output)
      (return (`NavigationSystem.K2_GetRandomReachablePointInRadius` (`self.K2_GetActorLocation` _output) 300.0))
      (else
        _)))
  (return (`NavigationSystem.K2_GetRandomReachablePointInRadius` (`self.K2_GetActorLocation`) (`self.Radius`))))

(fn `IsCharacterCanAdd`
  (params (S_CharacterData :type "/Game/MyGame/GameMode/GameData/S_CharacterData Structure (by ref)") (Mission :type Boolean) (Native :type Boolean))
  (returns (ReturnValue :type Boolean))
  (bind (_surname _name _camp _moral _constitution _strength _intelligence _health _damage _body _legs _occ _ismission_) (break `/Game/MyGame/GameMode/GameData/S_CharacterData` S_CharacterData))
  (return (and (or (== Native (not _ismission_)) (== _ismission_ Mission)) (> _health 0.0))))

(fn `IsPlayerInThisGuild?`
  (params (InActor :type "Actor Object Reference"))
  (returns (`In?` :type Boolean))
  (bind _asbp_game_mode_world_map (cast `/Game/MyGame/GameMode/Buleprint/BP_GameMode_WorldMap` (`GameplayStatics.GetGameMode`))
    (:`then`
      _)
    (:`CastFailed`
      _))
  (return (and (== InActor (`GameplayStatics.GetPlayerPawn` 0)) (== (`/Game/MyGame/GameMode/Buleprint/BP_GameMode_WorldMap.CurrGuildPoint` _asbp_game_mode_world_map) self))))

(fn `SelectNewCharacterLocation`
  (returns (ReturnValue :type "Vector Structure"))
  (bind _movepointarray (`self.MovePointArray`))
  (bind _output (`|GetArrayItem` _movepointarray (`KismetMathLibrary.RandomIntegerInRange` 0 (`KismetArrayLibrary.Array_LastIndex` _movepointarray))))
  (if (> (`KismetArrayLibrary.Array_Length` _movepointarray) 0)
    (`/Engine/EditorBlueprintResources/StandardMacros.IsValid` _output
      (:`Is Valid`
        (return (`NavigationSystem.K2_GetRandomReachablePointInRadius` (`self.K2_GetActorLocation` _output) 600.0)))
      (:`Is Not Valid`
        _)))
  (return (`NavigationSystem.K2_GetRandomReachablePointInRadius` (`self.K2_GetActorLocation`) (`self.Radius`))))

(fn `UserConstructionScript`
  (`parent.UserConstructionScript`)
  (bind _outactors (`GameplayStatics.GetAllActorsWithTag` (`KismetStringLibrary.Conv_StringToName` (`KismetStringLibrary.JoinStringArray` (`|MakeArray` "Guild" (`KismetStringLibrary.Conv_IntToString` (`self.GuildID`))) "_"))))
  (bind _output_get (set `self.MovePointArray` _outactors))
  (`KismetSystemLibrary.PrintString` (`KismetStringLibrary.Conv_IntToString` (`KismetArrayLibrary.Array_Length` _output_get))))