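; BP_GuildController lays out the world map's BP_GuildPoint actors on a staggered grid and assigns their GuildIDs.
; Its construction script fills an empty GuildActorArray, indexed by actor-name suffix, then positions each point eight-wide with odd rows offset.
; BeginPlay binds to the WorldMap game mode's guild-action-complete event, whose handler is empty.
; The DT_GuildData lookup is unused, and type-based sphere building is disconnected.
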(event `GuildActionComplate`
  (params (InGuildAction :type "/Game/MyGame/GameMode/GameData/S_GuildAction Structure")))

(event `self.ReceiveBeginPlay`
  (bind _asbp_game_mode_world_map (cast `/Game/MyGame/GameMode/Buleprint/BP_GameMode_WorldMap` (`GameplayStatics.GetGameMode`)))
  (add `/Game/MyGame/GameMode/Buleprint/BP_GameMode_WorldMap.ED_GuildActionComplate` _asbp_game_mode_world_map (delegate `GuildActionComplate`)))

(fn `SetGuildPointLocation`
  (params (InGuildID :type Integer) (GuildPoint :type "Actor Object Reference"))
  (bind (_outx _outy) (`/Game/MyGame/GameMode/Buleprint/BP_FunctionLibrary.GetGuildXY` InGuildID 8))
  (if (or (== _outy 1) (== _outy 3) (== _outy 5) (== _outy 7))
    (`self.K2_SetActorLocation` GuildPoint (`KismetMathLibrary.MakeVector` (+ (* _outx 51000.0) 38250.0) (+ (* _outy -51000.0) -25500.0) 30000.0) false false)
    (else
      (`self.K2_SetActorLocation` GuildPoint (`KismetMathLibrary.MakeVector` (+ (* _outx 51000.0) 12750.0) (+ (* _outy -51000.0) -25500.0) 30000.0) false false)))
  (bind _asbp_guild_point (cast `/Game/MyGame/GameMode/Buleprint/BP_GuildPoint` GuildPoint))
  (bind _output_get (set `/Game/MyGame/GameMode/Buleprint/BP_GuildPoint.GuildID` InGuildID _asbp_guild_point))
  (bind _returnvalue (`|GetDataTableRow` "/Game/MyGame/GameMode/GameData/DT_GuildData.DT_GuildData" (`KismetStringLibrary.Conv_StringToName` (`KismetStringLibrary.Conv_IntToString` _output_get)))))

(fn `UserConstructionScript`
  (if (<= (`KismetArrayLibrary.Array_Length` (`self.GuildActorArray`)) 0)
    (bind _outactors (`GameplayStatics.GetAllActorsOfClass` "/Game/MyGame/GameMode/Buleprint/BP_GuildPoint.BP_GuildPoint_C"))
    (for _array_element _outactors
      (`KismetArrayLibrary.Array_Set` (`self.GuildActorArray`) (`KismetStringLibrary.Conv_StringToInt` (`.RightS` (`KismetStringLibrary.Split` (`KismetSystemLibrary.GetObjectName` _array_element) "_" "IgnoreCase" "FromEnd"))) _array_element true))
    (for (_array_element_2 _array_index) (`self.GuildActorArray`)
      (`self.SetGuildPointLocation` _array_index _array_element_2))))