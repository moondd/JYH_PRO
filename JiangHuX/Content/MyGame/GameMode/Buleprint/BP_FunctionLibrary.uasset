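; Blueprint function library of shared helpers for guild, character and item data in a game with Confucian, Taoist and Buddhist sects.
; Shortcuts reach the game instance, world-map game mode and SaveGame guild array, with conversion between guild IDs and grid coordinates.
; Character creation draws surnames and male names from DataTables and derives health from attributes.
; Occupation follows guild type, faith and member index; item adding stacks goods, consumables and materials.
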(fn `AddItemToCharacter`
  (params (CharacterGuildID :type Integer) (CharacterChildID :type Integer) (Item :type "/Game/MyGame/GameMode/GameData/S_Item Structure"))
  (locals (Loc_Item :type "/Game/MyGame/GameMode/GameData/S_Item Structure") (Loc_CharacterItems :type "Array of /Game/MyGame/GameMode/GameData/S_Item Structure"))
  (bind _loc_item (`local.Loc_Item`))
  (bind _loc_characteritems (`local.Loc_CharacterItems`))
  (bind _output (`|GetArrayItem` _loc_characteritems (`KismetArrayLibrary.Array_Find` _loc_characteritems _loc_item)))
  (`|ExecutionSequence`
    (:`then_0`
      (set `local.Loc_Item` Item)
      (set `local.Loc_CharacterItems` (`.Items_111_C09E41C94CD2A43F4DD70A822C50FBD8` (break `/Game/MyGame/GameMode/GameData/S_CharacterData` (`self.GetCharacterData` CharacterGuildID CharacterChildID)))))
    (:`then_1`
      (switch `/Game/MyGame/GameMode/GameData/E_ItemType` (`.ItemType_5_69BEA3A542710826D715F8B02FC2CF83` (break `/Game/MyGame/GameMode/GameData/S_Item` _loc_item))
        (:`NewEnumerator0`
          (if (`KismetArrayLibrary.Array_Contains` _loc_characteritems _loc_item) :!label _label
            (setmembers `/Game/MyGame/GameMode/GameData/S_Item` :`StructRef` _output :`Amount` (+ (`.Amount_25_49A1739F46AB86814FA4EFA8B02205CA` (break `/Game/MyGame/GameMode/GameData/S_Item` _output)) (`.Amount_25_49A1739F46AB86814FA4EFA8B02205CA` (break `/Game/MyGame/GameMode/GameData/S_Item` _loc_item))))
            (else
              (`KismetArrayLibrary.Array_Add` _loc_characteritems _loc_item :!label _label_2))))
        (:`NewEnumerator1`
          (goto _label))
        (:`NewEnumerator4`
          (goto _label_2))
        (:`NewEnumerator2`
          (goto _label))
        (:`NewEnumerator5`
          (goto _label_2))
        (:`NewEnumerator3`
          (goto _label_2))
        (:`NewEnumerator6`
          (goto _label_2))))
    (:`then_2`
      (setmembers `/Game/MyGame/GameMode/GameData/S_CharacterData` :`StructRef` (`|GetArrayItem` (`.CharacterDataArray_77_471FFE724D5A30DA053F2387D6E7B8C9` (break `/Game/MyGame/GameMode/GameData/S_GuildData` (`|GetArrayItem` (`/Game/MyGame/GameMode/Buleprint/BP_SaveGame.GuildDataArray` (`self.GetMySaveGame` null)) CharacterGuildID))) CharacterChildID) :`Items` (`local.Loc_CharacterItems`)))))

(fn `GetCharacterData`
  (params (GuildID :type Integer) (CharacterID :type Integer))
  (returns (CharacterData :type "/Game/MyGame/GameMode/GameData/S_CharacterData Structure"))
  (bind _guilddataarray (`/Game/MyGame/GameMode/Buleprint/BP_SaveGame.GuildDataArray` (`self.GetMySaveGame` null)))
  (bind (_guildtype _name _ap _dominate _parentguildid _characterdataarray) (break `/Game/MyGame/GameMode/GameData/S_GuildData` (`|GetArrayItem` _guilddataarray GuildID)))
  (if (`KismetArrayLibrary.Array_IsValidIndex` _guilddataarray GuildID)
    (if (`KismetArrayLibrary.Array_IsValidIndex` _characterdataarray CharacterID)
      (return (`|GetArrayItem` _characterdataarray CharacterID))
      (else
        _)))
  (return))

(fn `GetCharacterOcc`
  (params (GuildType :type "/Game/MyGame/GameMode/GameData/E_GuildType Enum" :default "NewEnumerator0") (Faith :type "/Game/MyGame/GameMode/GameData/E_Faith Enum" :default "NewEnumerator0") (CharacterChildID :type Integer))
  (returns (Occ :type "/Game/MyGame/GameMode/GameData/E_CharacterOcc Enum"))
  (switch `/Game/MyGame/GameMode/GameData/E_GuildType` GuildType
    (:`NewEnumerator0`
      _)
    (:`NewEnumerator5`
      _)
    (:`NewEnumerator3`
      _)
    (:`NewEnumerator1`
      _)
    (:`NewEnumerator4`
      _)
    (:`NewEnumerator2`
      (switch `/Game/MyGame/GameMode/GameData/E_Faith` Faith
        (:`NewEnumerator0`
          (switch `int` CharacterChildID
            (:`Default`
              (return "NewEnumerator10"))
            (:`0`
              (return "NewEnumerator5"))
            (:`1`
              (return "NewEnumerator6"))
            (:`2`
              (return "NewEnumerator7"))
            (:`3`
              (return "NewEnumerator8"))
            (:`4`
              _)
            (:`5`
              _)
            (:`6`
              _))
          (return "NewEnumerator9"))
        (:`NewEnumerator1`
          (switch `int` CharacterChildID
            (:`Default`
              (return "NewEnumerator22"))
            (:`0`
              (return "NewEnumerator17"))
            (:`1`
              (return "NewEnumerator19"))
            (:`2`
              (return "NewEnumerator20"))
            (:`3`
              (return "NewEnumerator18"))
            (:`4`
              _)
            (:`5`
              _)
            (:`6`
              _))
          (return "NewEnumerator21"))
        (:`NewEnumerator2`
          (switch `int` CharacterChildID
            (:`Default`
              (return "NewEnumerator16"))
            (:`0`
              (return "NewEnumerator11"))
            (:`1`
              (return "NewEnumerator12"))
            (:`2`
              (return "NewEnumerator13"))
            (:`3`
              (return "NewEnumerator15"))
            (:`4`
              _)
            (:`5`
              _)
            (:`6`
              _))
          (return "NewEnumerator14")))))
  (return "NewEnumerator0"))

(fn `GetGameModeWorldMap`
  (returns (GameMode :type "/Game/MyGame/GameMode/Buleprint/BP_GameMode_WorldMap Object Reference"))
  (bind _asbp_game_mode_world_map (cast `/Game/MyGame/GameMode/Buleprint/BP_GameMode_WorldMap` (`GameplayStatics.GetGameMode` null)))
  (return _asbp_game_mode_world_map))

(fn `GetGuildDataWithID`
  (params (ID :type Integer))
  (returns (OutGuildID :type "/Game/MyGame/GameMode/GameData/S_GuildData Structure"))
  (return (`|GetArrayItem` (`/Game/MyGame/GameMode/Buleprint/BP_SaveGame.GuildDataArray` (`self.GetMySaveGame` null)) ID)))

(fn `GetGuildXY`
  (params (InGuildID :type Integer) (InWeight :type Integer :default 32))
  (returns (OutX :type Integer) (OutY :type Integer))
  (bind _returnvalue (/ InGuildID InWeight))
  (return (- InGuildID (* _returnvalue InWeight)) _returnvalue))

(fn `GetMyGameInstance`
  (returns (NewParam :type "/Game/MyGame/GameMode/Buleprint/BP_GameInstance Object Reference"))
  (bind _asbp_game_instance (cast `/Game/MyGame/GameMode/Buleprint/BP_GameInstance` (`GameplayStatics.GetGameInstance` null)))
  (return _asbp_game_instance))

(fn `GetMySaveGame`
  (returns (NewParam :type "/Game/MyGame/GameMode/Buleprint/BP_SaveGame Object Reference"))
  (return (`/Game/MyGame/GameMode/Buleprint/BP_GameInstance.SaveGame` (`self.GetMyGameInstance` null))))

(fn `GetParentGuildID`
  (params (GuildID :type Integer))
  (returns (ParentGuildID :type Integer))
  (return (`.ParentGuildID_79_CDE235094ECDDB4111764387B2601899` (break `/Game/MyGame/GameMode/GameData/S_GuildData` (`self.GetGuildDataWithID` GuildID)))))

(fn `GuildXYToID`
  (params (X :type Integer) (Y :type Integer) (Weight :type Integer :default 32))
  (returns (ID :type Integer))
  (return (+ (* Y Weight) X)))

(fn `RandomCharacterDataCreat`
  (params (Camp :type "/Game/MyGame/GameMode/GameData/E_Camp Enum" :default "NewEnumerator0") (Moral :type "/Game/MyGame/GameMode/GameData/E_Moral Enum" :default "NewEnumerator0"))
  (returns (OutCharacterData :type "/Game/MyGame/GameMode/GameData/S_CharacterData Structure"))
  (bind (_surname _name) (`self.RandomCharacterName` null))
  (bind _s_characterdata (make `/Game/MyGame/GameMode/GameData/S_CharacterData` _surname _name Camp Moral 0 0 0 30.0 6.0 "NewEnumerator0" false (`|MakeArray`)))
  (bind _maxhealth (`self.UnexpectedCharacterData` _s_characterdata))
  (bind _structout (setmembers `/Game/MyGame/GameMode/GameData/S_CharacterData` :`StructRef` _s_characterdata :`Health` _maxhealth))
  (return _structout))

(fn `RandomCharacterName`
  (returns (Surname :type Text) (Name :type Text))
  (`|ExecutionSequence`
    (:`then_0`
      (bind _outrownames (`DataTableFunctionLibrary.GetDataTableRowNames` "/Game/MyGame/GameMode/GameData/DT_Surname.DT_Surname"))
      (bind _returnvalue (`|GetDataTableRow` "/Game/MyGame/GameMode/GameData/DT_Surname.DT_Surname" (`|GetArrayItem` _outrownames (`KismetMathLibrary.RandomIntegerInRange` 0 (`KismetArrayLibrary.Array_LastIndex` _outrownames))))
        (:`RowNotFound`
          _)))
    (:`then_1`
      (bind _outrownames_2 (`DataTableFunctionLibrary.GetDataTableRowNames` "/Game/MyGame/GameMode/GameData/DT_Name_Male.DT_Name_Male"))
      (bind _returnvalue_2 (`|GetDataTableRow` "/Game/MyGame/GameMode/GameData/DT_Name_Male.DT_Name_Male" (`|GetArrayItem` _outrownames_2 (`KismetMathLibrary.RandomIntegerInRange` 0 (`KismetArrayLibrary.Array_LastIndex` _outrownames_2))))
        (:`RowNotFound`
          _)))
    (:`then_2`
      (return (`.Text_2_1D85C38040BA4BD0CB31C8B490EB547C` (break `/Game/MyGame/GameMode/GameData/S_Text` _returnvalue)) (`.Text_2_1D85C38040BA4BD0CB31C8B490EB547C` (break `/Game/MyGame/GameMode/GameData/S_Text` _returnvalue_2)))))
  (return "无" "名"))

(fn `UnexpectedCharacterData`
  (params (CharacterData :type "/Game/MyGame/GameMode/GameData/S_CharacterData Structure"))
  (returns (MaxHealth :type "Float (double-precision)") (Damage :type "Float (double-precision)") (ManaRecovery :type "Float (double-precision)"))
  (bind (_surname _name _camp _moral _constitution _strength _intelligence) (break `/Game/MyGame/GameMode/GameData/S_CharacterData` CharacterData))
  (return (+ 120.0 (* _constitution 0.6)) (+ 30.0 (* _strength 0.15)) (+ 15.0 (* _intelligence 0.075))))