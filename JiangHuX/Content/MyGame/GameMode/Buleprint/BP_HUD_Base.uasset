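; BP_HUD_Base is a HUD Blueprint that shows and hides the in-game, world map and player menu widgets.
; Each screen has a pair of custom events: Show creates the widget and adds it to the player screen only if none exists, and Hide removes it and clears the reference.
; BeginPlay is empty, so nothing appears until one of these events is called.
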(event `self.ReceiveBeginPlay`)

(event `Event_UI_Show_InGame`
  (`/Engine/EditorBlueprintResources/StandardMacros.IsValid` (`self.InGame`)
    (:`Is Not Valid`
      (bind _returnvalue (`|CreateWidget` "/Game/MyGame/UI/W_InGame.W_InGame_C"))
      (bind _output_get (set `self.InGame` _returnvalue))
      (`UserWidget.AddToPlayerScreen` _output_get 0))))

(event `Event_UI_Hide_InGame`
  (bind _ingame (`self.InGame`))
  (`/Engine/EditorBlueprintResources/StandardMacros.IsValid` _ingame
    (:`Is Valid`
      (`Widget.RemoveFromParent` _ingame)
      (set `self.InGame` null))))

(event `Event_UI_Show_WorldMap`
  (`/Engine/EditorBlueprintResources/StandardMacros.IsValid` (`self.WorldMap`)
    (:`Is Not Valid`
      (bind _returnvalue (`|CreateWidget` "/Game/MyGame/UI/W_WorldMap.W_WorldMap_C"))
      (bind _output_get (set `self.WorldMap` _returnvalue))
      (`UserWidget.AddToPlayerScreen` _output_get 0))))

(event `Event_UI_Hide_WorldMap`
  (bind _worldmap (`self.WorldMap`))
  (`/Engine/EditorBlueprintResources/StandardMacros.IsValid` _worldmap
    (:`Is Valid`
      (`Widget.RemoveFromParent` _worldmap)
      (set `self.WorldMap` null))))

(event `Event_UI_Show_PlayerMenu`
  (`/Engine/EditorBlueprintResources/StandardMacros.IsValid` (`self.PlayerMenu`)
    (:`Is Not Valid`
      (bind _returnvalue (`|CreateWidget` "/Game/MyGame/UI/W_PlayerMenu.W_PlayerMenu_C"))
      (bind _output_get (set `self.PlayerMenu` _returnvalue))
      (`UserWidget.AddToPlayerScreen` _output_get 0))))

(event `Event_UI_Hide_PlayerMenu`
  (bind _playermenu (`self.PlayerMenu`))
  (`/Engine/EditorBlueprintResources/StandardMacros.IsValid` _playermenu
    (:`Is Valid`
      (`Widget.RemoveFromParent` _playermenu)
      (set `self.PlayerMenu` null))))

(fn `UserConstructionScript`)