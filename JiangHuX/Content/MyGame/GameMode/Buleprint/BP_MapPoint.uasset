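; BP_MapPoint is a map location actor that detects when the player pawn enters or leaves its area.
; Overlapping the PlayerIn sphere calls EventPlayerIn, while ending overlap with the separate, tall PlayerExit volume calls EventPlayerLeave.
; An IsPlayerIn flag prevents repeated triggers.
; The construction script sizes both volumes from Radius; the Event_PlayerIn and Event_PlayerLeave handlers in this graph are empty.
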(event `self.PlayerIn.OnComponentBeginOverlap`
  (params (OverlappedComponent :type "PrimitiveComponent Object Reference") (OtherActor :type "Actor Object Reference") (OtherComp :type "PrimitiveComponent Object Reference") (OtherBodyIndex :type Integer) (bFromSweep :type Boolean) (SweepResult :type "HitResult Structure (by ref)"))
  (if (and (== OtherActor (`GameplayStatics.GetPlayerPawn` 0)) (not (`self.IsPlayerIn?`)))
    (set `self.IsPlayerIn?` true)
    (`self.Event_PlayerIn`)))

(event `self.PlayerExit.OnComponentEndOverlap`
  (params (OverlappedComponent :type "PrimitiveComponent Object Reference") (OtherActor :type "Actor Object Reference") (OtherComp :type "PrimitiveComponent Object Reference") (OtherBodyIndex :type Integer))
  (if (and (== OtherActor (`GameplayStatics.GetPlayerPawn` 0)) (`self.IsPlayerIn?`))
    (set `self.IsPlayerIn?` false)
    (`self.Event_PlayerLeave`)))

(event `Event_PlayerIn`)

(event `Event_PlayerLeave`)

(fn `UserConstructionScript`
  (bind _radius (`self.Radius`))
  (bind _playerin (`self.PlayerIn`))
  (bind _returnvalue (* _radius 0.03))
  (`SphereComponent.SetSphereRadius` _playerin _radius false)
  (`SceneComponent.K2_SetWorldLocation` _playerin (`self.K2_GetActorLocation`) false false)
  (`SceneComponent.K2_SetRelativeTransform` (`self.PlayerExit`) (`KismetMathLibrary.MakeTransform` (0.0 0.0 0.0) (struct) (`KismetMathLibrary.MakeVector` _returnvalue _returnvalue 100.0)) false false))